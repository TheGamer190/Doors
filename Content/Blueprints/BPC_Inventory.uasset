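; Inventory component that stores items as an array of item enums, with slots addressed by index.
; SetSlot writes an enum into a slot, and GetSlot resolves a slot's enum to its full row data through GetItemDetails.
; GetItemDetails does a linear scan of the DT_Items data table, returning the first row whose Enum field matches rather than looking up by row name.
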(fn `GetItemDetails`
  (params (requestedItem :type "/Game/Blueprints/E_Item Enum" :default "NewEnumerator0"))
  (returns (item :type "/Game/Blueprints/Structures/S_Item Structure"))
  (bind _outrownames (`DataTableFunctionLibrary.GetDataTableRowNames` "/Game/Blueprints/DataTables/DT_Items.DT_Items"))
  (for _array_element _outrownames
    (bind _returnvalue (`|GetDataTableRow` "/Game/Blueprints/DataTables/DT_Items.DT_Items" _array_element)
      (:`then`
        (if (`|EnumEquality` requestedItem (`.Enum_20_2D54A53A45602F5F55698992C840C854` (break `/Game/Blueprints/Structures/S_Item` _returnvalue)))
          (return _returnvalue))))))

(fn `GetSlot`
  (params (RequestedSlot :type Integer))
  (returns (`Item Details` :type "/Game/Blueprints/Structures/S_Item Structure"))
  (bind _item (`self.GetItemDetails` (`|GetArrayItem` (`self.enumInventory`) RequestedSlot)))
  (return _item))

(fn `SetSlot`
  (params (`Slot  Index` :type Integer) (Item :type "/Game/Blueprints/E_Item Enum" :default "NewEnumerator3"))
  (`KismetArrayLibrary.Array_Set` (`self.enumInventory`) `Slot  Index` Item))
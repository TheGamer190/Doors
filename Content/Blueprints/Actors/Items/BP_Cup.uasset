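; BP_Cup is a holdable item that captures and releases Pokémon.
; Use sphere-traces ahead of the camera, destroys a catchable BP_Pokemon and sets a captured flag; if no Pokémon is hit, it calls AltUse.
; AltUse activates Niagara, spawns a fresh BP_Pokemon ahead of the camera and clears the flag.
; Pickup disables collision and prints a key-found message, while Drop restores collision and physics with an impulse.
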(event `self.altUse`
  (bind _rootcomponent (`Actor.RootComponent` (`PlayerController.PlayerCameraManager` (`GameplayStatics.GetPlayerController` 0))))
  (if (`self.hasCapturedPokemon`)
    (`ActorComponent.Activate` (`self.Niagara`) false)
    (`|SpawnActorFromClass` "/Game/Blueprints/Actors/BP_Pokemon.BP_Pokemon_C" (`KismetMathLibrary.MakeTransform` (+ (`SceneComponent.K2_GetComponentLocation` _rootcomponent) (* (`SceneComponent.GetForwardVector` _rootcomponent) 300.0))) "Undefined" "MultiplyWithRoot" null null)
    (set `self.hasCapturedPokemon` false)
    (else
      (`KismetSystemLibrary.PrintText` "No pokemon captured!"))))

(event `self.Use`
  (bind _rootcomponent (`Actor.RootComponent` (`PlayerController.PlayerCameraManager` (`GameplayStatics.GetPlayerController` 0))))
  (bind _returnvalue (`SceneComponent.K2_GetComponentLocation` _rootcomponent))
  (bind _outhit (`KismetSystemLibrary.SphereTraceSingle` :`Start` _returnvalue :`End` (+ _returnvalue (* (`SceneComponent.GetForwardVector` _rootcomponent) 300.0)) :`TraceChannel` "TraceTypeQuery1" :`DrawDebugType` "ForDuration"))
  (bind _asbp_pokemon (cast `/Game/Blueprints/Actors/BP_Pokemon` (`.HitActor` (`GameplayStatics.BreakHitResult` _outhit)))
    (:`then`
      (if (`/Game/Blueprints/Actors/BP_Pokemon.canCatch` _asbp_pokemon)
        (`self.K2_DestroyActor` _asbp_pokemon)
        (set `self.hasCapturedPokemon` true)
        (else
          (`KismetSystemLibrary.PrintText` " \nTry feeding thhem first!"))))
    (:`CastFailed`
      (`/Game/Blueprints/BPI_Item.altUse`))))

(event `self.Drop`
  (bind _staticmesh (`self.StaticMesh`))
  (`PrimitiveComponent.SetCollisionEnabled` _staticmesh "QueryAndPhysics")
  (set `/Game/BPC_Interact.heldItem` null (stale `self.Pickup` owner))
  (`PrimitiveComponent.SetSimulatePhysics` _staticmesh true)
  (`PrimitiveComponent.AddImpulse` _staticmesh (200.0 0.0 50.0) "None" true))

(event `self.Pickup`
  (params (owner :type "/Game/BPC_Interact Object Reference"))
  (`KismetSystemLibrary.PrintText` "You found a key!")
  (`PrimitiveComponent.SetCollisionEnabled` (`self.StaticMesh`) "NoCollision"))

(fn `UserConstructionScript`)
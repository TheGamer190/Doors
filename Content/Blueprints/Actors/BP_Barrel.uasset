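; Barrel actor that opens when the first-person character enters its trigger sphere and shows its inventory.
; Sphere overlap begin and end call OpenBarrel, which plays or reverses a timeline that rotates the hinge component.
; On finishing an opening, it prints the first item's name and description and adds the chest menu widget, created at BeginPlay with the inventory, to the viewport.
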(event `self.Sphere.OnComponentBeginOverlap`
  (params (OverlappedComponent :type "PrimitiveComponent Object Reference") (OtherActor :type "Actor Object Reference") (OtherComp :type "PrimitiveComponent Object Reference") (OtherBodyIndex :type Integer) (bFromSweep :type Boolean) (SweepResult :type "HitResult Structure (by ref)"))
  (cast `/Game/FirstPerson/Blueprints/BP_FirstPersonCharacter` OtherActor)
  (`self.Open Barrel` false))

(event `self.ReceiveBeginPlay`
  (bind _returnvalue (`|CreateWidget` "/Game/UI/W_ChestMenu.W_ChestMenu_C" null (`self.Inventory`)))
  (set `self.chestMenu` _returnvalue))

(event `Open Barrel`
  (params (reverse :type Boolean))
  (bind (_name _description) (break `/Game/Blueprints/Structures/S_Item` (`|GetArrayItem` (`self.Inventory`))))
  (if reverse
    (bind (_direction _newtrack_0) (`Timeline|Timeline` :!via `Reverse` :!label _label)
      (:`Update`
        (`SceneComponent.K2_SetRelativeRotation` (`self.Hineg`) (`KismetMathLibrary.MakeRotator` (`KismetMathLibrary.Lerp` 0.0 -40.0 _newtrack_0)) false false))
      (:`Finished`
        (if (not reverse)
          (`KismetSystemLibrary.PrintText` (`|FormatText` "First item in the barrel is {name}. {Desc}" _name _description) true true (struct :`G` 0.66 :`B` 1.0 :`A` 1.0) 60.0)
          (`UserWidget.AddToViewport` (`self.chestMenu`) 0))))
    (else
      (goto _label))))

(event `self.Sphere.OnComponentEndOverlap`
  (params (OverlappedComponent :type "PrimitiveComponent Object Reference") (OtherActor :type "Actor Object Reference") (OtherComp :type "PrimitiveComponent Object Reference") (OtherBodyIndex :type Integer))
  (cast `/Game/FirstPerson/Blueprints/BP_FirstPersonCharacter` OtherActor)
  (`self.Open Barrel` true))

(fn `UserConstructionScript`)
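; BP_Beans is a holdable bean can that can make a Pokemon catchable or give the player an extra jump.
; Use sphere-traces from the camera, playing an eating sound and setting CanCatch on a hit BP_Pokemon, otherwise calling AltUse.
; AltUse briefly raises the jump limit, jumps, then destroys the can.
; Pickup disables collision and prints a key-found message, while Drop restores physics and applies a fixed impulse.
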(event `/Game/Blueprints/BPI_Item.Drop`
  (bind _can (`self.Can`))
  (`PrimitiveComponent.SetCollisionEnabled` _can "QueryAndPhysics")
  (set `/Game/BPC_Interact.heldItem` null (stale `/Game/Blueprints/BPI_Item.Pickup` owner))
  (`PrimitiveComponent.SetSimulatePhysics` _can true)
  (`PrimitiveComponent.AddImpulse` _can (200.0 0.0 50.0) "None" true))

(event `/Game/Blueprints/BPI_Item.Pickup`
  (params (owner :type "/Game/BPC_Interact Object Reference"))
  (`KismetSystemLibrary.PrintText` "You found a key!")
  (`PrimitiveComponent.SetCollisionEnabled` (`self.Can`) "NoCollision"))

(event `/Game/Blueprints/BPI_Item.altUse`
  (bind _asbp_first_person_character (cast `/Game/FirstPerson/Blueprints/BP_FirstPersonCharacter` (`GameplayStatics.GetPlayerCharacter` 0)))
  (set `Character.JumpMaxCount` 2 _asbp_first_person_character)
  (`Character.Jump` _asbp_first_person_character)
  (`KismetSystemLibrary.Delay` 0.2)
  (set `Character.JumpMaxCount` 1 _asbp_first_person_character)
  (`self.K2_DestroyActor`))

(event `/Game/Blueprints/BPI_Item.Use`
  (bind _rootcomponent (`Actor.RootComponent` (`PlayerController.PlayerCameraManager` (`GameplayStatics.GetPlayerController` 0))))
  (bind _returnvalue (`SceneComponent.K2_GetComponentLocation` _rootcomponent))
  (bind _outhit (`KismetSystemLibrary.SphereTraceSingle` :`Start` _returnvalue :`End` (+ _returnvalue (* (`SceneComponent.GetForwardVector` _rootcomponent) (`self.Dist`))) :`TraceChannel` "TraceTypeQuery1" :`DrawDebugType` "ForDuration"))
  (bind _asbp_pokemon (cast `/Game/Blueprints/Actors/BP_Pokemon` (`.HitActor` (`GameplayStatics.BreakHitResult` _outhit)))
    (:`then`
      (`GameplayStatics.PlaySoundAtLocation` "/Game/Audio/roblox-eating-sound-effect-nom-nom-nom.roblox-eating-sound-effect-nom-nom-nom" (`SceneComponent.K2_GetComponentLocation` (`self.Can`)) (struct) 1.0 1.0 0.0 null null null null)
      (set `/Game/Blueprints/Actors/BP_Pokemon.canCatch` true _asbp_pokemon))
    (:`CastFailed`
      (`/Game/Blueprints/BPI_Item.altUse`))))

(fn `UserConstructionScript`)
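; BP_Key is a holdable key item, an authentication card that opens BP_Door actors.
; Pickup prints a message and disables box and card collision, while Drop clears the owner's held item and throws the card with physics and an impulse.
; Use line-traces along the card's forward vector and, on hitting a door, clears the held slot, destroys the key and calls OpenDoor.
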(event `/Game/Blueprints/BPI_Item.Drop`
  (bind _authentication_card (`self.Authentication_Card`))
  (`PrimitiveComponent.SetCollisionEnabled` _authentication_card "QueryAndPhysics")
  (set `/Game/BPC_Interact.heldItem` null (stale `/Game/Blueprints/BPI_Item.Pickup` owner))
  (`PrimitiveComponent.SetSimulatePhysics` (`self.Authentication_Card`) true)
  (`PrimitiveComponent.AddImpulse` _authentication_card (200.0 0.0 50.0) "None" true))

(event `/Game/Blueprints/BPI_Item.Pickup`
  (params (owner :type "/Game/BPC_Interact Object Reference"))
  (`KismetSystemLibrary.PrintText` "You found a key!")
  (`PrimitiveComponent.SetCollisionEnabled` (`self.Box`) "NoCollision")
  (`PrimitiveComponent.SetCollisionEnabled` (`self.Authentication_Card`) "NoCollision"))

(event `/Game/Blueprints/BPI_Item.altUse`)

(event `/Game/Blueprints/BPI_Item.Use`
  (bind _authentication_card (`self.Authentication_Card`))
  (bind _returnvalue (`SceneComponent.K2_GetComponentLocation` _authentication_card))
  (bind _outhit (`KismetSystemLibrary.LineTraceSingle` _returnvalue (+ _returnvalue (* (`SceneComponent.GetForwardVector` _authentication_card) 300.0)) "TraceTypeQuery1"))
  (bind _asbp_door (cast `/Game/Blueprints/Actors/BP_Door` (`.HitActor` (`GameplayStatics.BreakHitResult` _outhit))))
  (set `/Game/BPC_Interact.heldItem` null (stale `/Game/Blueprints/BPI_Item.Pickup` owner))
  (`self.K2_DestroyActor`)
  (`/Game/Blueprints/Actors/BP_Door.OpenDoor` _asbp_door))

(fn `UserConstructionScript`)
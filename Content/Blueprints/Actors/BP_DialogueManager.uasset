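; Dialogue manager Blueprint that shows lines of dialogue on the first-person player's UI.
; Each DisplayNextLine call puts the current DialogueStrings entry in the UI's Dialogue text, advances the index, then clears the text after a short delay.
; Once the index reaches the end of the array, further calls only clear the text.
; Show and hide events reach the UI by casting the player character to BP_FirstPersonCharacter.
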(event `DisplayNextLine`
  (if (!= (`self.arrayIndex`) (`KismetArrayLibrary.Array_Length` (`self.dialogueStrings`)))
    (`self.ShowDialogue`)
    (`/Engine/EditorBlueprintResources/StandardMacros.IncrementInt` (`self.arrayIndex`)
      (:`  `
        (`KismetSystemLibrary.Delay` 1.5)
        (`self.HideDialogue`)))
    (else
      (`self.HideDialogue`))))

(event `ShowDialogue`
  (bind _asbp_first_person_character (cast `/Game/FirstPerson/Blueprints/BP_FirstPersonCharacter` (`GameplayStatics.GetPlayerCharacter` 0)))
  (`TextBlock.SetText` (`/Game/Blueprints/UW_Screen.Dialogue` (`/Game/FirstPerson/Blueprints/BP_FirstPersonCharacter.UI` _asbp_first_person_character)) (`|GetArrayItem` (`self.dialogueStrings`) (`self.arrayIndex`))))

(event `HideDialogue`
  (bind _asbp_first_person_character (cast `/Game/FirstPerson/Blueprints/BP_FirstPersonCharacter` (`GameplayStatics.GetPlayerCharacter` 0)))
  (`TextBlock.SetText` (`/Game/Blueprints/UW_Screen.Dialogue` (`/Game/FirstPerson/Blueprints/BP_FirstPersonCharacter.UI` _asbp_first_person_character)) ""))

(fn `UserConstructionScript`)
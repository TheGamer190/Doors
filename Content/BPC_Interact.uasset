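; Interaction component for BP_FirstPersonCharacter that lets the player pick up, use and drop items.
; After a short delay, IA_Interact sphere-traces from the camera, then sends Pickup to a BPI_Item actor and snaps it to HandHoldPoint as HeldItem.
; Debug keys E and left mouse send Drop and Use through the interface.
; TrytoPickUP repeats pickup for LastTouchedItem without setting HeldItem; older key-and-door trace logic is disconnected.
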(event Custom|TrytoPickUP
  (bind _last_touched_item (Variables|Default|Getlast%20Touched%20Item))
  (Utilities|IsValid _last_touched_item
    (:Is%20Valid
      (Class|BPIItem|Pickup(Message) _last_touched_item self)
      (Transformation|AttachComponentToComponent _last_touched_item (Variables|/Game/FirstPerson/Blueprints/BP_FirstPersonCharacter.BP_FirstPersonCharacter_C|GetHandHoldPoint (Variables|Default|GetPlayer)) "None" "SnapToTarget" "SnapToTarget" "KeepRelative" true))
    (:Is%20Not%20Valid
      (Development|PrintText "Nothing"))))

(event Input|EnhancedActionEvents|EnhancedInputActionIA_Interact
  (params (ActionValue :type Boolean) (ElapsedSeconds :type Float%20%28double-precision%29) (TriggeredSeconds :type Float%20%28double-precision%29) (InputAction :type Input%20Action%20Object%20Reference :default "/Game/Input/Actions/IA_Interact.IA_Interact"))
  (bind _returnvalue (Game|GetPlayerController 0))
  (bind _playercameramanager (Variables|/Script/Engine.PlayerController|GetPlayerCameraManager _returnvalue))
  (bind _rootcomponent (Variables|/Script/Engine.Actor|GetRootComponent _playercameramanager))
  (bind _returnvalue_2 (Transformation|GetWorldLocation _rootcomponent))
  (:Started
    (Utilities|FlowControl|Delay 0.2)
    (bind _outhit (Collision|SphereTraceByChannel _returnvalue_2 (+ _returnvalue_2 (* (Math|Vector|GetForwardVector _rootcomponent) (Variables|Default|GetLookDist))) 15.0 "TraceTypeQuery1" false 0 "ForDuration" true "(R=1.000000,G=0.000000,B=0.000000,A=1.000000)" "(R=0.000000,G=1.000000,B=0.000000,A=1.000000)" 1.0))
    (if true
      (if (Utilities|DoesObjectImplementInterface (.HitActor (Collision|BreakHitResult _outhit)) "/Game/Blueprints/BPI_Item.BPI_Item_C")
        (bind _output_get (Variables|Default|Setlast%20Touched%20Item (.HitActor (Collision|BreakHitResult _outhit))))
        (Development|PrintText (Utilities|Text|FormatText "Press F to pick up {name}." (Utilities|GetDisplayName (.HitActor (Collision|BreakHitResult _outhit)))))
        (Class|BPIItem|Pickup(Message) _output_get self)
        (Transformation|AttachComponentToComponent (Variables|Default|Getlast%20Touched%20Item) (Variables|/Game/FirstPerson/Blueprints/BP_FirstPersonCharacter.BP_FirstPersonCharacter_C|GetHandHoldPoint (Variables|Default|GetPlayer)) "None" "SnapToTarget" "SnapToTarget" "KeepRelative" true)
        (Variables|Default|SetheldItem (Variables|Default|Getlast%20Touched%20Item))
        (else
          (Variables|Default|Setlast%20Touched%20Item 0 :!label _label)))
      (else
        (goto _label)))))

(event EventBeginPlay
  (bind _asbp_first_person_character (Utilities|Casting|CastToBP_FirstPersonCharacter (Components|GetOwner)))
  (Variables|Default|SetPlayer _asbp_first_person_character)
  (Variables|Default|SetFirst%20Person%20Camera (Variables|/Game/FirstPerson/Blueprints/BP_FirstPersonCharacter.BP_FirstPersonCharacter_C|GetFirstPersonCamera _asbp_first_person_character)))

(event Input|KeyboardEvents|DebugKeyE
  (params (Key :type Key%20Structure :default "None") (ActionValue :type Input%20Action%20Value%20Structure))
  (:Pressed
    (Class|BPIItem|Drop(Message) (Variables|Default|GetheldItem))))

(event Input|MouseEvents|DebugKeyLeftMouseButton
  (params (Key :type Key%20Structure :default "None") (ActionValue :type Input%20Action%20Value%20Structure))
  (:Pressed
    (Class|BPIItem|Use(Message) (Variables|Default|GetheldItem))))